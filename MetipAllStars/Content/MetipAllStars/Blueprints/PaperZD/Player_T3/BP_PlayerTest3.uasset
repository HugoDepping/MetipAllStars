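; PaperZD test player character that moves along the X axis and forwards input to its animation instance.
; Light and heavy attacks send combo messages, while attack, charge attack, jumping and walking off ledges trigger animation node jumps.
; Sprint changes walk speed and run animation play rate together.
; Hard-wired number keys request a damaged state or swap the attack sequence before jumping to a shared dynamic attack node.
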(event `InputAxis|MoveRight`
  (params (AxisValue :type "Float (single-precision)"))
  (`self.AddMovementInput` (1.0 0.0 0.0) AxisValue))

(event `InputAction|LightAttack`
  (params (Key :type "Key Structure"))
  (:`Pressed`
    (message `/Game/MetipAllStars/Blueprints/PaperZD/Combo/BP_ComboRequest.RequestCombo` (`PaperZDAnimationComponent.AnimInstance` (`self.AnimationComponent`)) "NewEnumerator0")))

(event `InputAction|Jump`
  (params (Key :type "Key Structure"))
  (:`Pressed`
    (`self.Jump`)))

(event `InputAction|HeavyAttack`
  (params (Key :type "Key Structure"))
  (:`Pressed`
    (message `/Game/MetipAllStars/Blueprints/PaperZD/Combo/BP_ComboRequest.RequestCombo` (`PaperZDAnimationComponent.AnimInstance` (`self.AnimationComponent`)) "NewEnumerator1")))

(event `self.OnJumped`
  (`PaperZDAnimInstance.JumpToNode` (`PaperZDAnimationComponent.AnimInstance` (`self.AnimationComponent`)) "JumpActivated" "None" :!label _label))

(event `Key|Four`
  (params (Key :type "Key Structure"))
  (:`Pressed`
    (message `/Game/MetipAllStars/Blueprints/PaperZD/Combo/BPI_StateRequest.JumpStateRequest` (`PaperZDAnimationComponent.AnimInstance` (`self.AnimationComponent`)) "Damaged" "New State Machine")))

(event `self.OnWalkingOffLedge`
  (params (PreviousFloorImpactNormal :type "Vector Structure (by ref)") (PreviousFloorContactNormal :type "Vector Structure (by ref)") (PreviousLocation :type "Vector Structure (by ref)") (TimeDelta :type "Float (single-precision)"))
  (goto _label))

(event `InputAction|ChargeAttack`
  (params (Key :type "Key Structure"))
  (:`Pressed`
    (set `self.Charging` true)
    (`PaperZDAnimInstance.JumpToNode` (`PaperZDAnimationComponent.AnimInstance` (`self.AnimationComponent`)) "ChargeAttack" "None"))
  (:`Released`
    (set `self.Charging` false)))

(event `InputAction|Attack`
  (params (Key :type "Key Structure"))
  (:`Pressed`
    (`PaperZDAnimInstance.JumpToNode` (`PaperZDAnimationComponent.AnimInstance` (`self.AnimationComponent`)) "Attack" "None")))

(event `InputAction|Sprint`
  (params (Key :type "Key Structure"))
  (bind _charactermovement (`self.CharacterMovement`))
  (bind _animinstance (`PaperZDAnimationComponent.AnimInstance` (`self.AnimationComponent`)))
  (:`Pressed`
    (set `CharacterMovementComponent.MaxWalkSpeed` 600.0 _charactermovement)
    (bind _asanim_bp_character (cast `/Game/MetipAllStars/Blueprints/PaperZD/Tutorial/AnimBP_Character` _animinstance))
    (set `/Game/MetipAllStars/Blueprints/PaperZD/Tutorial/AnimBP_Character.RunPlayRate` 2.0 _asanim_bp_character))
  (:`Released`
    (set `CharacterMovementComponent.MaxWalkSpeed` 300.0 _charactermovement)
    (bind _asanim_bp_character_2 (cast `/Game/MetipAllStars/Blueprints/PaperZD/Tutorial/AnimBP_Character` _animinstance))
    (set `/Game/MetipAllStars/Blueprints/PaperZD/Tutorial/AnimBP_Character.RunPlayRate` 1.0 _asanim_bp_character_2)))

(event `Key|Five`
  (params (Key :type "Key Structure"))
  (bind _animinstance (`PaperZDAnimationComponent.AnimInstance` (`self.AnimationComponent`)))
  (:`Pressed`
    (bind _asanim_bp_character (cast `/Game/MetipAllStars/Blueprints/PaperZD/Tutorial/AnimBP_Character` _animinstance))
    (set `/Game/MetipAllStars/Blueprints/PaperZD/Tutorial/AnimBP_Character.AttackSequenceAnimation` "/Game/MetipAllStars/Blueprints/PaperZD/Tutorial/AnimSequences/NA_Straight.NA_Straight" _asanim_bp_character)
    (`PaperZDAnimInstance.JumpToNode` _animinstance "DynamicAttackJump" "New State Machine")))

(event `Key|Six`
  (params (Key :type "Key Structure"))
  (bind _animinstance (`PaperZDAnimationComponent.AnimInstance` (`self.AnimationComponent`)))
  (:`Pressed`
    (bind _asanim_bp_character (cast `/Game/MetipAllStars/Blueprints/PaperZD/Tutorial/AnimBP_Character` _animinstance))
    (set `/Game/MetipAllStars/Blueprints/PaperZD/Tutorial/AnimBP_Character.AttackSequenceAnimation` "/Game/MetipAllStars/Blueprints/PaperZD/Tutorial/AnimSequences/NA_Up.NA_Up" _asanim_bp_character)
    (`PaperZDAnimInstance.JumpToNode` _animinstance "DynamicAttackJump" "New State Machine")))

(fn `UserConstructionScript`)