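; Paper2D player character base that handles side-to-side walking and jumping with Hugo flipbook animations.
; On BeginPlay it adds the default Enhanced Input mapping context through BP_PlayerControls.
; Movement input drives the walk or idle flipbook and rotates the sprite to face the travel direction, but is ignored mid-jump.
; Jumping plays a non-looping flipbook, then a delay loop polls for zero vertical velocity to restore idle and unlock input.
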(event `self.ReceiveBeginPlay`
  (bind _asbp_player_controls (cast `/Game/MetipAllStars/Blueprints/Character/BP_PlayerControls` (`self.GetController`)))
  (`EnhancedInputSubsystemInterface.AddMappingContext` (pcsubsystem `EnhancedInputLocalPlayerSubsystem` _asbp_player_controls) "/Game/MetipAllStars/Blueprints/Character/IMC_Default.IMC_Default" 0 (struct)))

(event `EnhancedInput|/Game/MetipAllStars/Blueprints/Character/IA_Movement`
  (params (ActionValue :type "Float (double-precision)") (ElapsedSeconds :type "Float (double-precision)") (TriggeredSeconds :type "Float (double-precision)") (InputAction :type "InputAction Object Reference" :default "/Game/MetipAllStars/Blueprints/Character/IA_Movement.IA_Movement"))
  (:`Triggered`
    (if (not (`self.isJumping`))
      (`self.AddMovementInput` (`self.GetActorForwardVector`) ActionValue)
      (`PaperFlipbookComponent.SetFlipbook` (`self.Sprite`) "/Game/MetipAllStars/Characters/Prototype_2/04_Walk_Jump/01_Walk/01_Walk_Hugo.01_Walk_Hugo")
      (`SceneComponent.K2_SetWorldRotation` (`self.Sprite`) (select `bool` (> ActionValue 0.0) :`false` (struct :`Yaw` -180.0) :`true` (struct) :!type "Rotator Structure") false false)))
  (:`Completed`
    (if (not (`self.isJumping`))
      (`PaperFlipbookComponent.SetFlipbook` (`self.Sprite`) "/Game/MetipAllStars/Characters/Prototype_2/01_Idle/02_Idle/01_Idle_Hugo.01_Idle_Hugo"))))

(event `EnhancedInput|/Game/MetipAllStars/Blueprints/Character/IA_Jump`
  (params (ActionValue :type Boolean) (ElapsedSeconds :type "Float (double-precision)") (TriggeredSeconds :type "Float (double-precision)") (InputAction :type "InputAction Object Reference" :default "/Game/MetipAllStars/Blueprints/Character/IA_Jump.IA_Jump"))
  (bind (_returnvalue_x _returnvalue_y _returnvalue_z) (`KismetMathLibrary.BreakVector` (`self.GetVelocity`)))
  (bind _sprite (`self.Sprite`))
  (:`Triggered`
    (if (not (`self.isJumping`))
      (set `self.isJumping` true)
      (`self.Jump`)
      (`PaperFlipbookComponent.SetLooping` _sprite false)
      (`PaperFlipbookComponent.SetFlipbook` _sprite "/Game/MetipAllStars/Characters/Prototype_2/04_Walk_Jump/02_Jump/02_Jump_Hugo.02_Jump_Hugo")
      (`KismetSystemLibrary.Delay` 0.1)
      (if (== _returnvalue_z 0.0) :!label _label
        (`PaperFlipbookComponent.SetLooping` _sprite true)
        (`PaperFlipbookComponent.Play` _sprite)
        (`PaperFlipbookComponent.SetFlipbook` _sprite "/Game/MetipAllStars/Characters/Prototype_2/01_Idle/02_Idle/01_Idle_Hugo.01_Idle_Hugo")
        (set `self.isJumping` false)
        (else
          (`KismetSystemLibrary.Delay` 0.1)
          (goto _label))))))

(fn `UserConstructionScript`)