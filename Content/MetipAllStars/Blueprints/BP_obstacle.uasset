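; BP_obstacle is an obstacle that, when Hit is called, gets shoved along X and falls once no ground is beneath it.
; A Timeline drives a swept relative offset, scaled by MoveStrength, with its direction taken from the sign of the cube's rounded world X.
; Each update also traces downward from the cube, enabling physics simulation when nothing is hit and disabling it otherwise.
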(event `self.ReceiveHit`
  (params (MyComp :type "PrimitiveComponent Object Reference") (Other :type "Actor Object Reference") (OtherComp :type "PrimitiveComponent Object Reference") (bSelfMoved :type Boolean) (HitLocation :type "Vector Structure") (HitNormal :type "Vector Structure") (NormalImpulse :type "Vector Structure") (Hit :type "HitResult Structure (by ref)"))
  (bind _returnvalue (`SceneComponent.K2_GetComponentLocation` (`self.Cube`)))
  (bind _returnvalue_x (`KismetMathLibrary.BreakVector` (`SceneComponent.K2_GetComponentLocation` (`self.Cube`))))
  (bind (_direction _lerp_0_1) (`Timeline|Timeline` :!via `PlayFromStart`)
    (:`Update`
      (`SceneComponent.K2_AddRelativeLocation` (`self.DefaultSceneRoot`) (`KismetMathLibrary.VLerp` (`KismetMathLibrary.MakeVector` (* (`self.MoveStrength`) (`KismetMathLibrary.Clamp` (`KismetMathLibrary.Round` _returnvalue_x) -1 1))) (0.0 0.0 0.0) _lerp_0_1) true false)
      (bind (_outhit _returnvalue_2) (`KismetSystemLibrary.LineTraceSingleByProfile` _returnvalue (+ _returnvalue (0.0 0.0 -400.0))))
      (`PrimitiveComponent.SetSimulatePhysics` (`self.Cube`) (not _returnvalue_2)))))

(fn `UserConstructionScript`)