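; BP_ItemBase is a pickup item actor whose effect type comes from its Itemstates value.
; Any overlap with CollisionBox calls ItemPickedUp, as the branch condition is fixed to true and the overlapping actor is not checked.
; ItemPickedUp switches on speed, health increase, health restore, paralyze and shoot, then destroys the item.
; The effects are placeholders that only print debug strings.
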(event `self.CollisionBox.OnComponentBeginOverlap`
  (params (OverlappedComponent :type "PrimitiveComponent Object Reference") (OtherActor :type "Actor Object Reference") (OtherComp :type "PrimitiveComponent Object Reference") (OtherBodyIndex :type Integer) (bFromSweep :type Boolean) (SweepResult :type "HitResult Structure (by ref)"))
  (if true
    (`/Game/MetipAllStars/Blueprints/PickUpSystem/I_PickUpItem.ItemPickedUp` (`self.Itemstates`))
    (else
      (`KismetSystemLibrary.PrintString` (`KismetSystemLibrary.GetDisplayName` OtherActor)))))

(event `/Game/MetipAllStars/Blueprints/PickUpSystem/I_PickUpItem.ItemPickedUp`
  (params (ItemState :type "/Game/MetipAllStars/Blueprints/PickUpSystem/Enum/E_ItemStates Enum" :default "NewEnumerator0"))
  (switch `/Game/MetipAllStars/Blueprints/PickUpSystem/Enum/E_ItemStates` ItemState
    (:`NewEnumerator0`
      (`KismetSystemLibrary.PrintString` "Speed Called"))
    (:`NewEnumerator1`
      (`KismetSystemLibrary.PrintString` "Increase Health Called"))
    (:`NewEnumerator4`
      (`KismetSystemLibrary.PrintString` "Restore Health Called"))
    (:`NewEnumerator2`
      (`KismetSystemLibrary.PrintString` "Paralyze Called"))
    (:`NewEnumerator3`
      (`KismetSystemLibrary.PrintString` "Shoot Called")))
  (`self.K2_DestroyActor`))

(fn `UserConstructionScript`)