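; Item spawner actor for the pickup system that periodically drops a random item inside a box volume.
; Tick drives a latent Delay of random length, from a fixed minimum up to MaximumTime, which acts as a repeating timer.
; When it completes, SpawnItem spawns a random class from ItemBaseArray at a random point within the Box bounds, then a debug string prints.
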(event `self.ReceiveTick`
  (params (DeltaSeconds :type "Float (single-precision)"))
  (`KismetSystemLibrary.Delay` (`KismetMathLibrary.RandomFloatInRange` 30.0 (`self.MaximumTime`)))
  (`self.SpawnItem` (`KismetArrayLibrary.Array_Random` (`self.ItemBaseArray`)))
  (`KismetSystemLibrary.PrintString` "IEEEEEee"))

(fn `SpawnItem`
  (params (ItemToSpawn :type "Actor Class Reference"))
  (bind (_origin _boxextent) (`KismetSystemLibrary.GetComponentBounds` (`self.Box`)))
  (`|SpawnActorFromClass` ItemToSpawn (`KismetMathLibrary.MakeTransform` (`KismetMathLibrary.RandomPointInBoundingBox` _origin _boxextent)) "Undefined" "MultiplyWithRoot" null null))

(fn `UserConstructionScript`)